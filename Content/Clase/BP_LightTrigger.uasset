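; BP_LightTrigger is a light trigger that pairs a SpotLight with a Sphere overlap volume.
; The SpotLight is hidden in game at BeginPlay, and any begin overlap calls NewFunction, which sets its color to black without checking the actor.
; End overlap calls SelfLightVisibility, whose body is empty, so nothing in this graph makes the light visible again.
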(event `self.ReceiveBeginPlay`
  (`SceneComponent.SetHiddenInGame` (`self.SpotLight`) true false))

(event `self.Sphere.OnComponentBeginOverlap`
  (params (OverlappedComponent :type "PrimitiveComponent Object Reference") (OtherActor :type "Actor Object Reference") (OtherComp :type "PrimitiveComponent Object Reference") (OtherBodyIndex :type Integer) (bFromSweep :type Boolean) (SweepResult :type "HitResult Structure (by ref)"))
  (`self.NewFunction` OtherActor))

(event `self.Sphere.OnComponentEndOverlap`
  (params (OverlappedComponent :type "PrimitiveComponent Object Reference") (OtherActor :type "Actor Object Reference") (OtherComp :type "PrimitiveComponent Object Reference") (OtherBodyIndex :type Integer))
  (`self.SelfLightVisibility` OtherActor))

(fn `NewFunction`
  (params (Object :type "Object Object Reference"))
  (`LightComponent.SetLightColor` :`self` (`self.SpotLight`)))

(fn `SelfLightVisibility`
  (params (Object :type "Object Object Reference") (NewHidden :type Boolean)))

(fn `UserConstructionScript`)